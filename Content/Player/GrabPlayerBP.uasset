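; Player Blueprint that can grab objects through a Grabber component and auto-follow actors tagged SimClient.
; Grab input selects on press and grabs on release, while raise and drop inputs tilt the Grabber each tick.
; Holding Follow cycles highlighted candidates; releasing starts SimpleMoveToActor pursuit, halting within reach distance and cancelled by manual movement.
; Control rotation eases toward the actor's facing on input or while following in motion.
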(event `InputAction|RaiseGrabber`
  (params (Key :type "Key Structure"))
  ;[1 1 1] Grabbing
  (:`Pressed`
    (set `self.GrabTiltSpeed` 0.8))
  (:`Released`
    (set `self.GrabTiltSpeed` 0.0 :!label _label)))

(event `InputAction|OrientViewportToActor`
  (params (Key :type "Key Structure"))
  ;[1 1 1] Orient Viewport
  (:`Pressed`
    (set `self.OrientViewport` true))
  (:`Released`
    (set `self.OrientViewport` false)))

(event `InputAction|DropGrabber`
  (params (Key :type "Key Structure"))
  ;[1 1 1] Grabbing
  (:`Pressed`
    (set `self.GrabTiltSpeed` -0.8))
  (:`Released`
    (goto _label)))

(event `InputAction|Grab`
  (params (Key :type "Key Structure"))
  (bind _grabber (`self.Grabber`))
  (bind _grabber_2 (`self.Grabber`))
  ;[1 1 1] Grabbing
  (:`Pressed`
    (if (`Grabber.isGrabbing` (`self.Grabber`))
      (`Grabber.UnGrab` _grabber)
      (set `self.ToGrab` false)
      (else
        (`Grabber.SelectStart` _grabber)
        (set `self.ToGrab` true))))
  (:`Released`
    (if (`self.ToGrab`)
      (`Grabber.Grab` _grabber_2)
      (`Grabber.SelectEnd` _grabber_2))))

(event `FollowStart_Event`
  (params (TargetActor :type "Actor Object Reference"))
  ;[1 1 1] Follow Start/End Event handler for debugging
  (`KismetSystemLibrary.PrintString` (`KismetSystemLibrary.GetObjectName` TargetActor)))

(event `self.ReceiveTick`
  (params (DeltaSeconds :type "Float (single-precision)"))
  ;[1 1 1] Tick
  (set `self.DeltaTime` DeltaSeconds)
  (`|ExecutionSequence`
    (:`then_0`
      (`self.ProcessOrientViewport`))
    (:`then_1`
      (`Grabber.TiltGrabber` (`self.Grabber`) (`self.GrabTiltSpeed`)))
    (:`then_2`
      (`self.CheckAbortFollowing`))
    (:`then_3`
      (if (`self.Following`)
        (if (>= (`self.ReachDistance`) (`self.GetDistanceTo` (`self.FollowActor`) self))
          (`NavMovementComponent.StopActiveMovement` (`self.CharacterMovement`))
          (else
            (`AIBlueprintHelperLibrary.SimpleMoveToActor` (`self.GetController`) (`self.FollowActor`))))))))

(event `FollowEnd_Event`
  ;[1 1 1] Follow Start/End Event handler for debugging
  (`NavMovementComponent.StopActiveMovement` (`self.CharacterMovement`))
  (`KismetSystemLibrary.PrintString` "Follow End Event"))

(event `InputAction|Follow`
  (params (Key :type "Key Structure"))
  ;[1 1 1] Following target selection
  (:`Pressed`
    (`|ExecutionSequence`
      (:`then_0`
        (bind _outactors (`GameplayStatics.GetAllActorsWithTag` "SimClient"))
        (set `self.FollowCandidate` _outactors))
      (:`then_1`
        (set `self.FollowSelecting` true))
      (:`then_2`
        (if (`self.Following`)
          (set `self.FollowSelectionID` -1)
          (else
            (bind _result (`/Engine/EditorBlueprintResources/StandardMacros.DecrementInt` (`KismetArrayLibrary.Array_Length` (`self.FollowCandidate`)))
              (:`  `
                (set `self.FollowSelectionID` _result))))))
      (:`then_3`
        (set `self.SelectionChange` 0)
        (`self.UpdateSelection`))))
  (:`Released`
    (`|ExecutionSequence`
      (:`then_0`
        (set `self.FollowSelecting` false))
      (:`then_1`
        (if (`self.Following`)
          (`self.EndFollowing`)
          (elif (>= (`self.FollowSelectionID`) 0)
            (bind _output_get (set `self.FollowActor` (`|GetArrayItem` (`self.FollowCandidate`) (`self.FollowSelectionID`))))
            (set `self.Following` true)
            (`self.FollowStart_Event` _output_get)))))))

(event `InputAction|SelectUp`
  (params (Key :type "Key Structure"))
  ;[1 1 1] Following target selection
  (:`Pressed`
    (set `self.SelectionChange` 1)
    (`self.UpdateSelection` :!label _label_2)))

(event `InputAction|SelectDown`
  (params (Key :type "Key Structure"))
  ;[1 1 1] Following target selection
  (:`Pressed`
    (set `self.SelectionChange` -1)
    (goto _label_2)))

(fn `CheckAbortFollowing`
  (if (or (> (`KismetMathLibrary.Abs` (`self.GetInputAxisValue`)) 0.01) (> (`KismetMathLibrary.Abs` (`self.GetInputAxisValue`)) 0.01) (> (`KismetMathLibrary.Abs` (`self.GetInputAxisValue`)) 0.01))
    (if (`self.Following`)
      (`self.EndFollowing`))))

(fn `EndFollowing`
  (`Grabber.Unhilight` (`self.Grabber`))
  (set `self.FollowActor` null)
  (set `self.Following` false)
  (`self.FollowEnd_Event`))

(fn `ProcessOrientViewport`
  (bind _returnvalue (`GameplayStatics.GetPlayerController` 0))
  (bind _returnvalue_2 (`Controller.GetControlRotation` _returnvalue))
  (if (or (`self.OrientViewport`) (and (`self.Following`) (> (`KismetMathLibrary.VSize` (`self.GetVelocity`)) 0.0)))
    (`Controller.SetControlRotation` _returnvalue (`KismetMathLibrary.RInterpTo` _returnvalue_2 (`KismetMathLibrary.MakeRotator` (.roll (`self.K2_GetActorRotation`)) (.pitch _returnvalue_2) (.yaw (`self.K2_GetActorRotation`))) (`self.DeltaTime`) 8.0))))

(fn `UpdateSelection`
  (bind _returnvalue (`KismetArrayLibrary.Array_Length` (`self.FollowCandidate`)))
  (if (`self.FollowSelecting`)
    (if (`KismetMathLibrary.Conv_IntToBool` _returnvalue)
      (bind _output_get (set `self.FollowSelectionID` (mod (+ (`self.FollowSelectionID`) (`self.SelectionChange`) _returnvalue) _returnvalue)))
      (`Grabber.HilightActor` (`self.Grabber`) (`|GetArrayItem` (`self.FollowCandidate`) _output_get))
      (else
        (set `self.FollowSelectionID` -1)))))

(fn `UserConstructionScript`)